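; BP_DCharacter is a character Blueprint that keeps a camera helper component on its capsule.
; Every Tick it draws a debug sphere at the helper's location, then re-attaches the helper to the capsule, snapping location and keeping relative rotation and scale.
; A vertical-velocity check and a few related nodes are left disconnected, and the construction script is empty.
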(event `self.ReceiveTick`
  (params (DeltaSeconds :type "Float (single-precision)"))
  (`KismetSystemLibrary.DrawDebugSphere` (`SceneComponent.GetSocketLocation` (`self.CameraHelperComponent`) "None") 10.0 12 (struct :`R` 1.0 :`B` 0.86875 :`A` 1.0) 0.0 2.0)
  (`SceneComponent.K2_AttachToComponent` (`self.CameraHelperComponent`) (`self.CapsuleComponent`) "None" "SnapToTarget" "KeepRelative" "KeepRelative" true))

(fn `UserConstructionScript`)